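; Letter puzzle mini-game actor where the player drags fifteen torn letter pieces into place with the mouse under a dedicated camera.
; Clicked pieces follow the deprojected cursor at fixed height; each release checks every piece against its tag-matched target in XY within a small tolerance.
; Solving, or pressing L, plays UI stages and reveals the whole letter.
; Ending marks the clue found, switches day lighting to night, restores the camera and destroys the actor.
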(event `Key|L`
  (params (Key :type "Key Structure"))
  (bind _puzzlegameui (`self.PuzzleGameUI`))
  (:`Pressed`
    ;[0.1773 1 0.3373] Завершение пазла
    (`/Game/MiniGames/Letter_puzzle/UI/UI_PuzzleGame.All Puzzles Solved` _puzzlegameui :!label _label)
    (`KismetSystemLibrary.Delay` 3.0)
    (`/Game/MiniGames/Letter_puzzle/UI/UI_PuzzleGame.Fade` _puzzlegameui)
    (`KismetSystemLibrary.Delay` 3.0)
    (`/Game/MiniGames/Letter_puzzle/UI/UI_PuzzleGame.Final Stage` _puzzlegameui)
    (for _array_element (`|MakeArray` (`self.LetterPiece_01`) (`self.LetterPiece_02`) (`self.LetterPiece_03`) (`self.LetterPiece_04`) (`self.LetterPiece_05`) (`self.LetterPiece_06`) (`self.LetterPiece_07`) (`self.LetterPiece_08`) (`self.LetterPiece_09`) (`self.LetterPiece_10`) (`self.LetterPiece_11`) (`self.LetterPiece_12`) (`self.LetterPiece_13`) (`self.LetterPiece_14`) (`self.LetterPiece_15`) (`self.Hint`))
      (`ActorComponent.K2_DestroyComponent` _array_element))
    (`SceneComponent.SetVisibility` (`self.AllLetter`) true false)))

(event `Solved`
  ;[0.1773 1 0.3373] Завершение пазла
  (goto _label))

(event `self.LetterPiece_02.OnReleased`
  (params (TouchedComponent :type "PrimitiveComponent Object Reference") (ButtonReleased :type "Key Structure"))
  ;[0.6007 0.09194 1] Подбор и отпускание кусочков письма
  (`self.On Released Component`))

(event `self.LetterPiece_01.OnClicked`
  (params (TouchedComponent :type "PrimitiveComponent Object Reference") (ButtonPressed :type "Key Structure"))
  ;[0.6007 0.09194 1] Подбор и отпускание кусочков письма
  (`self.On Clicked Component` TouchedComponent))

(event `self.LetterPiece_01.OnReleased`
  (params (TouchedComponent :type "PrimitiveComponent Object Reference") (ButtonReleased :type "Key Structure"))
  ;[0.6007 0.09194 1] Подбор и отпускание кусочков письма
  (`self.On Released Component`))

(event `self.LetterPiece_02.OnClicked`
  (params (TouchedComponent :type "PrimitiveComponent Object Reference") (ButtonPressed :type "Key Structure"))
  ;[0.6007 0.09194 1] Подбор и отпускание кусочков письма
  (`self.On Clicked Component` TouchedComponent))

(event `self.LetterPiece_04.OnClicked`
  (params (TouchedComponent :type "PrimitiveComponent Object Reference") (ButtonPressed :type "Key Structure"))
  ;[0.6007 0.09194 1] Подбор и отпускание кусочков письма
  (`self.On Clicked Component` TouchedComponent))

(event `self.LetterPiece_03.OnClicked`
  (params (TouchedComponent :type "PrimitiveComponent Object Reference") (ButtonPressed :type "Key Structure"))
  ;[0.6007 0.09194 1] Подбор и отпускание кусочков письма
  (`self.On Clicked Component` TouchedComponent))

(event `self.LetterPiece_03.OnReleased`
  (params (TouchedComponent :type "PrimitiveComponent Object Reference") (ButtonReleased :type "Key Structure"))
  ;[0.6007 0.09194 1] Подбор и отпускание кусочков письма
  (`self.On Released Component`))

(event `self.LetterPiece_04.OnReleased`
  (params (TouchedComponent :type "PrimitiveComponent Object Reference") (ButtonReleased :type "Key Structure"))
  ;[0.6007 0.09194 1] Подбор и отпускание кусочков письма
  (`self.On Released Component`))

(event `self.LetterPiece_05.OnClicked`
  (params (TouchedComponent :type "PrimitiveComponent Object Reference") (ButtonPressed :type "Key Structure"))
  ;[0.6007 0.09194 1] Подбор и отпускание кусочков письма
  (`self.On Clicked Component` TouchedComponent))

(event `self.LetterPiece_06.OnClicked`
  (params (TouchedComponent :type "PrimitiveComponent Object Reference") (ButtonPressed :type "Key Structure"))
  ;[0.6007 0.09194 1] Подбор и отпускание кусочков письма
  (`self.On Clicked Component` TouchedComponent))

(event `self.LetterPiece_05.OnReleased`
  (params (TouchedComponent :type "PrimitiveComponent Object Reference") (ButtonReleased :type "Key Structure"))
  ;[0.6007 0.09194 1] Подбор и отпускание кусочков письма
  (`self.On Released Component`))

(event `self.LetterPiece_06.OnReleased`
  (params (TouchedComponent :type "PrimitiveComponent Object Reference") (ButtonReleased :type "Key Structure"))
  ;[0.6007 0.09194 1] Подбор и отпускание кусочков письма
  (`self.On Released Component`))

(event `self.LetterPiece_08.OnClicked`
  (params (TouchedComponent :type "PrimitiveComponent Object Reference") (ButtonPressed :type "Key Structure"))
  ;[0.6007 0.09194 1] Подбор и отпускание кусочков письма
  (`self.On Clicked Component` TouchedComponent))

(event `self.LetterPiece_07.OnClicked`
  (params (TouchedComponent :type "PrimitiveComponent Object Reference") (ButtonPressed :type "Key Structure"))
  ;[0.6007 0.09194 1] Подбор и отпускание кусочков письма
  (`self.On Clicked Component` TouchedComponent))

(event `self.ReceiveTick`
  (params (DeltaSeconds :type "Float (single-precision)"))
  (bind (_worldlocation _worlddirection) (`PlayerController.DeprojectMousePositionToWorld` (`GameplayStatics.GetPlayerController` 0)))
  ;[1 0.5961 0.2872] Проверка и передвиждение кусочков письма
  (if (`self.bIsDragging`)
    (`SceneComponent.K2_SetWorldLocation` (`self.DraggedPiece`) (`KismetMathLibrary.MakeVector` (.x (+ _worldlocation (* _worlddirection (`KismetMathLibrary.Conv_DoubleToVector` 140.0)))) (.y (+ _worldlocation (* _worlddirection (`KismetMathLibrary.Conv_DoubleToVector` 140.0)))) (+ 102.0 5.0)) false false)))

(event `self.LetterPiece_08.OnReleased`
  (params (TouchedComponent :type "PrimitiveComponent Object Reference") (ButtonReleased :type "Key Structure"))
  ;[0.6007 0.09194 1] Подбор и отпускание кусочков письма
  (`self.On Released Component`))

(event `self.LetterPiece_07.OnReleased`
  (params (TouchedComponent :type "PrimitiveComponent Object Reference") (ButtonReleased :type "Key Structure"))
  ;[0.6007 0.09194 1] Подбор и отпускание кусочков письма
  (`self.On Released Component`))

(event `self.LetterPiece_10.OnClicked`
  (params (TouchedComponent :type "PrimitiveComponent Object Reference") (ButtonPressed :type "Key Structure"))
  ;[0.6007 0.09194 1] Подбор и отпускание кусочков письма
  (`self.On Clicked Component` TouchedComponent))

(event `self.LetterPiece_09.OnClicked`
  (params (TouchedComponent :type "PrimitiveComponent Object Reference") (ButtonPressed :type "Key Structure"))
  ;[0.6007 0.09194 1] Подбор и отпускание кусочков письма
  (`self.On Clicked Component` TouchedComponent))

(event `self.LetterPiece_10.OnReleased`
  (params (TouchedComponent :type "PrimitiveComponent Object Reference") (ButtonReleased :type "Key Structure"))
  ;[0.6007 0.09194 1] Подбор и отпускание кусочков письма
  (`self.On Released Component`))

(event `self.LetterPiece_09.OnReleased`
  (params (TouchedComponent :type "PrimitiveComponent Object Reference") (ButtonReleased :type "Key Structure"))
  ;[0.6007 0.09194 1] Подбор и отпускание кусочков письма
  (`self.On Released Component`))

(event `Start mini-game`
  (bind _returnvalue (`GameplayStatics.GetPlayerController` 0))
  (bind _puzzlegameui (`self.PuzzleGameUI`))
  ;[1 1 1] Запуск мини-игры
  (`self.EnableInput` _returnvalue)
  (bind _returnvalue_2 (`|CreateWidget` (`self.UI_PuzzleGame`)))
  (bind _output_get (set `self.PuzzleGameUI` _returnvalue_2))
  (`UserWidget.AddToViewport` _output_get 0)
  (`PlayerController.SetViewTargetWithBlend` _returnvalue (`ActorComponent.GetOwner` (`self.MinigameCamera`)) 0.0 "VTBlend_Linear" 0.0 false)
  (set `PlayerController.bShowMouseCursor` true _returnvalue)
  (set `PlayerController.bEnableMouseOverEvents` true _returnvalue)
  (`WidgetBlueprintLibrary.SetInputMode_GameAndUIEx` _returnvalue _puzzlegameui "DoNotLock" false)
  (bind _outactors (`GameplayStatics.GetAllActorsOfClass` "/Game/MiniGames/Letter_puzzle/Blueprints/BP_Letter.BP_Letter_C"))
  (bind _output (`|GetArrayItem` _outactors))
  (set `/Game/MiniGames/Letter_puzzle/Blueprints/BP_Letter.bIsInteractableLetter` false _output)
  (set `/Game/MiniGames/Letter_puzzle/Blueprints/BP_Letter.bIsPlayerInRange` false _output)
  (`/Game/MiniGames/Letter_puzzle/UI/UI_PuzzleGame.HideHint` _puzzlegameui))

(event `self.LetterPiece_12.OnClicked`
  (params (TouchedComponent :type "PrimitiveComponent Object Reference") (ButtonPressed :type "Key Structure"))
  ;[0.6007 0.09194 1] Подбор и отпускание кусочков письма
  (`self.On Clicked Component` TouchedComponent))

(event `self.LetterPiece_11.OnClicked`
  (params (TouchedComponent :type "PrimitiveComponent Object Reference") (ButtonPressed :type "Key Structure"))
  ;[0.6007 0.09194 1] Подбор и отпускание кусочков письма
  (`self.On Clicked Component` TouchedComponent))

(event `self.LetterPiece_12.OnReleased`
  (params (TouchedComponent :type "PrimitiveComponent Object Reference") (ButtonReleased :type "Key Structure"))
  ;[0.6007 0.09194 1] Подбор и отпускание кусочков письма
  (`self.On Released Component`))

(event `self.LetterPiece_11.OnReleased`
  (params (TouchedComponent :type "PrimitiveComponent Object Reference") (ButtonReleased :type "Key Structure"))
  ;[0.6007 0.09194 1] Подбор и отпускание кусочков письма
  (`self.On Released Component`))

(event `self.LetterPiece_14.OnClicked`
  (params (TouchedComponent :type "PrimitiveComponent Object Reference") (ButtonPressed :type "Key Structure"))
  ;[0.6007 0.09194 1] Подбор и отпускание кусочков письма
  (`self.On Clicked Component` TouchedComponent))

(event `self.LetterPiece_13.OnClicked`
  (params (TouchedComponent :type "PrimitiveComponent Object Reference") (ButtonPressed :type "Key Structure"))
  ;[0.6007 0.09194 1] Подбор и отпускание кусочков письма
  (`self.On Clicked Component` TouchedComponent))

(event `End Mini-Game`
  (bind _returnvalue (`GameplayStatics.GetPlayerController` 0))
  (bind _returnvalue_2 (`GameplayStatics.GetPlayerController` 0))
  (bind _returnvalue_3 (`GameplayStatics.GetGameInstance`))
  ;[1 0.1713 0.1614] Завершение мини-игры
  (message `/Game/dopros/BPI_GetClue.MarkClueAsFound` _returnvalue_3 "Letter")
  (`KismetSystemLibrary.Delay` 2.0)
  (`Widget.RemoveFromParent` (`self.PuzzleGameUI`))
  (bind _asbp_game_instance (cast `/Game/GameInstance/BP_GameInstance` _returnvalue_3))
  (`/Game/GameInstance/BP_GameInstance.ShowLoadingScreen` _asbp_game_instance)
  (set `PlayerController.bShowMouseCursor` false _returnvalue)
  (set `PlayerController.bEnableMouseOverEvents` false _returnvalue)
  (`WidgetBlueprintLibrary.SetInputMode_GameOnly` _returnvalue)
  (bind _outactors (`GameplayStatics.GetAllActorsOfClassWithTag` "/Script/Engine.DirectionalLight" "Day"))
  (`SceneComponent.SetVisibility` (`Light.LightComponent` (`|GetArrayItem` _outactors)) false false)
  (bind _outactors_2 (`GameplayStatics.GetAllActorsOfClassWithTag` "/Script/Engine.DirectionalLight" "Night"))
  (`SceneComponent.SetVisibility` (`Light.LightComponent` (`|GetArrayItem` _outactors_2)) true false)
  (bind _outactors_3 (`GameplayStatics.GetAllActorsOfClass` "/Game/MiniGames/Letter_puzzle/Blueprints/BP_Letter.BP_Letter_C"))
  (`/Game/MiniGames/Letter_puzzle/Blueprints/BP_Letter.LetterView` (`|GetArrayItem` _outactors_3))
  (bind _current_camera (`/Game/GameInstance/BP_GameInstance.Current Camera` _asbp_game_instance))
  (if (`KismetSystemLibrary.IsValid` _current_camera)
    (`PlayerController.SetViewTargetWithBlend` _returnvalue_2 _current_camera 0.0 "VTBlend_Linear" 0.0 false)
    (else
      (bind _asbp_gojbase_character (cast `/Game/Player/BP_GOJBaseCharacter` (`self.BP_GOJChar`)))
      (`PlayerController.SetViewTargetWithBlend` _returnvalue_2 _asbp_gojbase_character 0.0 "VTBlend_Linear" 0.0 false)))
  (`KismetSystemLibrary.Delay` 3.0)
  (`/Game/GameInstance/BP_GameInstance.CloseLoadingScreen` _asbp_game_instance)
  (`self.K2_DestroyActor`))

(event `self.LetterPiece_14.OnReleased`
  (params (TouchedComponent :type "PrimitiveComponent Object Reference") (ButtonReleased :type "Key Structure"))
  ;[0.6007 0.09194 1] Подбор и отпускание кусочков письма
  (`self.On Released Component`))

(event `self.LetterPiece_13.OnReleased`
  (params (TouchedComponent :type "PrimitiveComponent Object Reference") (ButtonReleased :type "Key Structure"))
  ;[0.6007 0.09194 1] Подбор и отпускание кусочков письма
  (`self.On Released Component`))

(event `self.LetterPiece_15.OnClicked`
  (params (TouchedComponent :type "PrimitiveComponent Object Reference") (ButtonPressed :type "Key Structure"))
  ;[0.6007 0.09194 1] Подбор и отпускание кусочков письма
  (`self.On Clicked Component` TouchedComponent))

(event `self.LetterPiece_15.OnReleased`
  (params (TouchedComponent :type "PrimitiveComponent Object Reference") (ButtonReleased :type "Key Structure"))
  ;[0.6007 0.09194 1] Подбор и отпускание кусочков письма
  (`self.On Released Component`))

(event `self.ReceiveBeginPlay`
  (bind _outactors (`GameplayStatics.GetAllActorsOfClassWithTag` "/Script/Engine.DirectionalLight" "Day"))
  (`SceneComponent.SetVisibility` (`Light.LightComponent` (`|GetArrayItem` _outactors)) true false)
  (bind _outactors_2 (`GameplayStatics.GetAllActorsOfClassWithTag` "/Script/Engine.DirectionalLight" "Night"))
  (`SceneComponent.SetVisibility` (`Light.LightComponent` (`|GetArrayItem` _outactors_2)) false false))

(fn `CheckPuzzleCompletion`
  (returns (AllPuzzleOnPlace :type Boolean))
  (for _array_element (`|MakeArray` (`self.LetterPiece_01`) (`self.LetterPiece_02`) (`self.LetterPiece_03`) (`self.LetterPiece_04`) (`self.LetterPiece_05`) (`self.LetterPiece_06`) (`self.LetterPiece_07`) (`self.LetterPiece_08`) (`self.LetterPiece_09`) (`self.LetterPiece_10`) (`self.LetterPiece_11`) (`self.LetterPiece_12`) (`self.LetterPiece_13`) (`self.LetterPiece_14`) (`self.LetterPiece_15`))
    (set `self.bMatchFound` false)
    (for _array_element_2 (`|MakeArray` (`self.TargetPosition_1`) (`self.TargetPosition_2`) (`self.TargetPosition_3`) (`self.TargetPosition_4`) (`self.TargetPosition_5`) (`self.TargetPosition_6`) (`self.TargetPosition_7`) (`self.TargetPosition_8`) (`self.TargetPosition_9`) (`self.TargetPosition_10`) (`self.TargetPosition_11`) (`self.TargetPosition_12`) (`self.TargetPosition_13`) (`self.TargetPosition_14`) (`self.TargetPosition_15`))
      (bind _output (`|GetArrayItem` (`ActorComponent.ComponentTags` _array_element_2)))
      (if (== _output (`|GetArrayItem` (`ActorComponent.ComponentTags` _array_element)))
        (`KismetSystemLibrary.PrintString` (`KismetStringLibrary.Conv_NameToString` _output))
        (bind (_returnvalue_x _returnvalue_y) (`KismetMathLibrary.BreakVector` (`SceneComponent.K2_GetComponentLocation` _array_element_2)))
        (bind (_returnvalue_x_2 _returnvalue_y_2) (`KismetMathLibrary.BreakVector` (`SceneComponent.K2_GetComponentLocation` _array_element)))
        (bind _returnvalue (`KismetMathLibrary.VSize` (- (`KismetMathLibrary.MakeVector` _returnvalue_x _returnvalue_y) (`KismetMathLibrary.MakeVector` _returnvalue_x_2 _returnvalue_y_2))))
        (`KismetSystemLibrary.PrintString` (`KismetStringLibrary.Conv_DoubleToString` _returnvalue))
        (if (<= _returnvalue 2.0)
          (set `self.bMatchFound` true)
          (break))))
    (if (`self.bMatchFound`)
      (set `self.bMatchFound` false)
      (else
        (return false))))
  (return true))

(fn `On Clicked Component`
  (params (Object :type "Object Object Reference"))
  (`GameplayStatics.PlaySound2D` "/Game/MiniGames/Letter_puzzle/Sounds/paper-up.paper-up" 1.0 1.0 0.0 null null)
  (bind _asstatic_mesh_component (cast `StaticMeshComponent` Object))
  (set `self.DraggedPiece` _asstatic_mesh_component)
  (set `self.bIsDragging` true))

(fn `On Released Component`
  (bind _draggedpiece (`self.DraggedPiece`))
  (bind (_returnvalue_x _returnvalue_y _returnvalue_z) (`KismetMathLibrary.BreakVector` (`SceneComponent.K2_GetComponentLocation` _draggedpiece)))
  (if (`KismetSystemLibrary.IsValid` _draggedpiece)
    (`GameplayStatics.PlaySound2D` "/Game/MiniGames/Letter_puzzle/Sounds/paper-down.paper-down" 1.0 1.0 0.0 null null)
    (`SceneComponent.K2_SetWorldLocation` _draggedpiece (`KismetMathLibrary.MakeVector` _returnvalue_x _returnvalue_y (- _returnvalue_z 3.0)) false false)
    (set `self.DraggedPiece` null)
    (set `self.bIsDragging` false)
    (bind _allpuzzleonplace (`self.CheckPuzzleCompletion`))
    (if _allpuzzleonplace
      (`KismetSystemLibrary.PrintString` "удалось")
      (`self.Solved`)
      (else
        (`KismetSystemLibrary.PrintString` "не все на месте")))))

(fn `UserConstructionScript`)